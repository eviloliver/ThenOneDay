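; Boss AI controller that runs its default behavior tree and tracks the player through AI perception.
; On BeginPlay it starts the tree and stores player pawn 0 as the blackboard target.
; Sensing an MJPlayerCharacter sets IsSeeingTarget and adds a test boss HP bar widget to that player's viewport, with a debug print.
; Any failed-sense update clears the flag and removes the widget.
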(event `self.ReceiveBeginPlay`
  (`self.RunBehaviorTree` (`BehaviorTreeComponent.DefaultBehaviorTreeAsset` (`self.BehaviorTreeComponent`)))
  (`BlackboardComponent.SetValueAsObject` (`self.Blackboard`) (`self.TargetActorKey`) (`GameplayStatics.GetPlayerPawn` 0)))

(event `self.AIPerceptionComponent.OnTargetPerceptionUpdated`
  (params (Actor :type "Actor Object Reference") (Stimulus :type "AIStimulus Structure"))
  (bind _isseeingtarget (`self.IsSeeingTarget`))
  (bind _blackboard (`self.Blackboard`))
  (if (`.bSuccessfullySensed` (break `AIStimulus` Stimulus))
    (bind _asmjplayer_character (cast `MJPlayerCharacter` Actor))
    (`BlackboardComponent.SetValueAsBool` _blackboard _isseeingtarget true)
    (bind _asbp_mjplayer_controller (cast `/Game/Core/Controller/BP_MJPlayerController` (`Pawn.GetController` _asmjplayer_character)))
    (bind _returnvalue (`|CreateWidget` "/Game/TG/AI/WBP_AIBossHpBarTest.WBP_AIBossHpBarTest_C" _asbp_mjplayer_controller))
    (`UserWidget.AddToViewport` _returnvalue 0)
    (`KismetSystemLibrary.PrintText` "Detect!")
    (else
      (`BlackboardComponent.SetValueAsBool` _blackboard _isseeingtarget false)
      (`/Game/TG/AI/WBP_AIBossHpBarTest.Event RemoveFromParent` _returnvalue))))

(fn `UserConstructionScript`)