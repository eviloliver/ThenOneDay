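; Boss plane projectile actor that flies an arced path over a set time, then destroys itself.
; Each Tick lerps from start to end location by elapsed time and adds a sine-shaped offset along the actor's up vector, scaled by Height.
; The Initialize event sets both start and end location from its single StartLocation input.
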(event `self.ReceiveTick`
  (params (DeltaSeconds :type "Float (single-precision)"))
  ;[1 1 1] Updating Location
  (bind _output_get (set `self.Elapsed` (+ (`self.Elapsed`) DeltaSeconds)))
  (bind _output_get_2 (set `self.Alpha` (/ _output_get (`self.Time`))))
  (`self.K2_SetActorLocation` (+ (* (`self.GetActorUpVector`) (* (`KismetMathLibrary.Sin` (`KismetMathLibrary.MultiplyByPi` _output_get_2)) (`self.Height`))) (`KismetMathLibrary.VLerp` (`self.StartLocation`) (`self.EndLocation`) (`self.Alpha`))))
  (if (>= (`self.Elapsed`) (`self.Time`))
    (`self.K2_DestroyActor`)))

(event `Initialize`
  (params (StartLocation :type "Vector Structure"))
  ;[1 1 1] Expose on Spawn
  (set `self.StartLocation` StartLocation)
  (set `self.EndLocation` StartLocation))

(fn `UserConstructionScript`)