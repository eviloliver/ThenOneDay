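; Test portal actor in town that sends the player into the generated dungeon when anything overlaps its collision.
; Overlap generates the dungeon graph via MJDungeonGenerationSubSystem, caches the town game mode and player session data, then plays a 2D sound.
; When the sound finishes, the current map number's graph node selects a Battle, Reward or Boss chunk map, and the game mode travels there with that node's ID.
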(event `AudioEnd`
  (bind (_nodeid _assignedmapid _nodetype) (break `MJDungeonNode` (`|GetArrayItem` (`.Nodes` (break `MJDungeonGraph` (`MJDungeonGenerationSubSystem.DungeonGraph` (subsystem `MJDungeonGenerationSubSystem`)))) (`KismetMathLibrary.Conv_ByteToInt` (`.CurrentDungeonMapNum` (break `MJPlayerSessionData` (stale `self.Collision.OnComponentBeginOverlap` _returnvalue)))))))
  (switch `EMJNodeType` _nodetype
    (:`Battle`
      (`MJGameModeBase.TravelToMapByNode` (stale `self.Collision.OnComponentBeginOverlap` _asbp_gamemode_town_tg) (`KismetTextLibrary.Conv_TextToString` (`|FormatText` "Dungeon_Chunk_Battle0{0}" (`KismetMathLibrary.Conv_IntToByte` _assignedmapid))) (`KismetMathLibrary.Conv_IntToByte` _nodeid)))
    (:`Reward`
      (`MJGameModeBase.TravelToMapByNode` (stale `self.Collision.OnComponentBeginOverlap` _asbp_gamemode_town_tg) (`KismetTextLibrary.Conv_TextToString` (`|FormatText` "Dungeon_Chunk_Reward")) (`KismetMathLibrary.Conv_IntToByte` _nodeid)))
    (:`Boss`
      (`MJGameModeBase.TravelToMapByNode` (stale `self.Collision.OnComponentBeginOverlap` _asbp_gamemode_town_tg) (`KismetTextLibrary.Conv_TextToString` (`|FormatText` "Dungeon_Chunk_Boss")) (`KismetMathLibrary.Conv_IntToByte` _nodeid)))))

(event `self.Collision.OnComponentBeginOverlap`
  (params (OverlappedComponent :type "PrimitiveComponent Object Reference") (OtherActor :type "Actor Object Reference") (OtherComp :type "PrimitiveComponent Object Reference") (OtherBodyIndex :type Integer) (bFromSweep :type Boolean) (SweepResult :type "HitResult Structure (by ref)"))
  (`|ExecutionSequence`
    (:`then_0`
      (`MJDungeonGenerationSubSystem.GenerateDungeonGraph` (subsystem `MJDungeonGenerationSubSystem`)))
    (:`then_1`
      (bind _asbp_gamemode_town_tg (cast `/Game/Core/GameMode/BP_Gamemode_Town_TG` (`GameplayStatics.GetGameMode`)))
      (bind _asmjgame_instance_tg (cast `MJGameInstanceTG` (`GameplayStatics.GetGameInstance`))
        (:`then`
          (`KismetSystemLibrary.PrintText` "Travel to DugeonStartnode!!" true true (struct :`R` 1.0 :`G` 0.073746 :`A` 1.0))
          (bind _returnvalue (`MJGameInstanceTG.GetPlayerSessionDataRef` _asmjgame_instance_tg))
          (bind _returnvalue_2 (`GameplayStatics.SpawnSound2D` "/Game/SFX_Asset/Game/Game_Test.Game_Test" 1.0 1.0 0.0 null))
          (add `AudioComponent.OnAudioFinished` _returnvalue_2 (delegate `AudioEnd`)))
        (:`CastFailed`
          (`KismetSystemLibrary.PrintText` "Cast Failed!"))))))

(fn `UserConstructionScript`)