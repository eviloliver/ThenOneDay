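; BP_TestPortalToNextDungeon is a test portal actor that brings up the player's map widget while the player stands on it.
; On sphere overlap with BP_TG_MJPlayerCharacter, it sets the character's IsOnPortal flag, then has its map widget draw edges and graph and become visible.
; On end overlap it clears the flag and hides the widget if visible.
; The Blueprint itself contains no travel logic.
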(event `self.Sphere.OnComponentBeginOverlap`
  (params (OverlappedComponent :type "PrimitiveComponent Object Reference") (OtherActor :type "Actor Object Reference") (OtherComp :type "PrimitiveComponent Object Reference") (OtherBodyIndex :type Integer) (bFromSweep :type Boolean) (SweepResult :type "HitResult Structure (by ref)"))
  (bind _asbp_tg_mjplayer_character (cast `/Game/TG/BP_TG_MJPlayerCharacter` OtherActor))
  (set `/Game/TG/BP_TG_MJPlayerCharacter.bIsOnPortal` true _asbp_tg_mjplayer_character)
  (bind _mapwidgetref (`/Game/TG/BP_TG_MJPlayerCharacter.MapWidgetRef` _asbp_tg_mjplayer_character))
  (`/Game/TG/TestWBP/WBP_DungeonMapTest.DrawEdge` _mapwidgetref)
  (`/Game/TG/TestWBP/WBP_DungeonMapTest.DrawGraph` _mapwidgetref)
  (`/Game/TG/TestWBP/WBP_DungeonMapTest.SetAllVisibility` _mapwidgetref "Visible"))

(event `self.Sphere.OnComponentEndOverlap`
  (params (OverlappedComponent :type "PrimitiveComponent Object Reference") (OtherActor :type "Actor Object Reference") (OtherComp :type "PrimitiveComponent Object Reference") (OtherBodyIndex :type Integer))
  (bind _asbp_tg_mjplayer_character (cast `/Game/TG/BP_TG_MJPlayerCharacter` OtherActor))
  (set `/Game/TG/BP_TG_MJPlayerCharacter.bIsOnPortal` false _asbp_tg_mjplayer_character)
  (bind _mapwidgetref (`/Game/TG/BP_TG_MJPlayerCharacter.MapWidgetRef` _asbp_tg_mjplayer_character))
  (if (`Widget.IsVisible` _mapwidgetref)
    (`/Game/TG/TestWBP/WBP_DungeonMapTest.SetAllVisibility` _mapwidgetref "Hidden")))

(fn `UserConstructionScript`)