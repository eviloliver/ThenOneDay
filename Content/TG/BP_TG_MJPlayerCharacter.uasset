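; Player character Blueprint with debug hotkeys for testing dungeon AI and the boss.
; Keys delete spawned AI through the dungeon GameState, place a dummy actor in front of the player, toggle a dungeon map widget, and publish boss health changes.
; Another key cycles the boss state enum, and BossToPhase writes it to the boss AI controller's Blackboard.
; BeginPlay creates the boss HP bar widget and keeps it hidden.
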(event `Key|I`
  (params (Key :type "Key Structure"))
  (:`Pressed`
    (bind _asbp_game_state_dungeon (cast `/Game/Core/GameState/BP_GameState_Dungeon` (`GameplayStatics.GetGameState`)))
    (`self.K2_DestroyActor` (`|GetArrayItem` (`MJGameStateDungeonTG.SpawnedActorRefs` _asbp_game_state_dungeon) (`self.DeleteAINum`)))
    (`KismetSystemLibrary.PrintText` "Delete Actor")
    (`/Engine/EditorBlueprintResources/StandardMacros.IncrementInt` (`self.DeleteAINum`)
      (:`  `
        (`/Engine/EditorBlueprintResources/StandardMacros.DecrementInt` (`MJGameStateDungeonTG.CurrSpawnedAINum` _asbp_game_state_dungeon))))))

(event `Key|L`
  (params (Key :type "Key Structure"))
  ;[1 1 1] Place Actor
  (:`Pressed`
    (`|SpawnActorFromClass` "/Game/TG/Actor/BP_DummyActor_TG.BP_DummyActor_TG_C" (`KismetMathLibrary.Conv_VectorToTransform` (+ (`self.K2_GetActorLocation`) (* (`KismetMathLibrary.GetForwardVector` (`self.GetControlRotation`)) 100.0))) "Undefined" "MultiplyWithRoot" null null)))

(event `Key|M`
  (params (Key :type "Key Structure"))
  ;[1 1 1] Map Toggle
  (:`Pressed`
    (bind _output_get (set `self.MapButtonPressed` (not (`self.MapButtonPressed`))))
    (if _output_get
      (bind _asbp_mjplayer_controller (cast `/Game/Core/Controller/BP_MJPlayerController` (`self.GetController` self)))
      (bind _returnvalue (`|CreateWidget` "/Game/TG/MapTestWBP/WBP_DungeonMapTest.WBP_DungeonMapTest_C" _asbp_mjplayer_controller))
      (`UserWidget.AddToViewport` _returnvalue 0)
      (`/Game/TG/MapTestWBP/WBP_DungeonMapTest.DrawGraph` _returnvalue)
      (else
        (`Widget.RemoveFromParent` _returnvalue)))))

(event `Key|P`
  (params (Key :type "Key Structure"))
  ;[1 1 1] Change Boss State
  (:`Pressed`
    (bind _result (`/Engine/EditorBlueprintResources/StandardMacros.IncrementInt` (`KismetMathLibrary.Conv_ByteToInt` (`self.Input State`)))
      (:`  `
        (bind _output_get (set `self.Input State` (cast `/Game/TG/AI/BPENUM_BossState` (`KismetMathLibrary.Conv_IntToByte` (mod _result (enumcount `/Game/TG/AI/BPENUM_BossState`))))))
        (`self.BossToPhase` _output_get)))))

(event `Key|O`
  (params (Key :type "Key Structure"))
  ;[1 1 1] Damage To Boss
  (:`Pressed`
    (bind _asmjgame_state_dungeon_tg (cast `MJGameStateDungeonTG` (`GameplayStatics.GetGameState`)))
    (`MJGameStateDungeonTG.PublishOnBossHealthChanged` _asmjgame_state_dungeon_tg 21.0)))

(event `self.ReceiveBeginPlay`
  ;[1 1 1] BeginPlay
  (bind _asbp_mjplayer_controller (cast `/Game/Core/Controller/BP_MJPlayerController` (`self.GetController`)))
  (bind _returnvalue (`|CreateWidget` "/Game/TG/AI/WBP_AIBossHpBarTest.WBP_AIBossHpBarTest_C" _asbp_mjplayer_controller))
  (`UserWidget.AddToViewport` _returnvalue 0)
  (set `self.BossHPWidgetClass` _returnvalue)
  (`Widget.SetVisibility` _returnvalue "Hidden"))

(fn `BossToPhase`
  (params (InputState :type "/Game/TG/AI/BPENUM_BossState Enum" :default "NewEnumerator1"))
  (bind _returnvalue (`GameplayStatics.GetActorOfClass` "/Game/TG/AI/BP_AIBossCharacter.BP_AIBossCharacter_C"))
  (`KismetSystemLibrary.PrintString` (`KismetTextLibrary.Conv_TextToString` (`|FormatText` "Boss Phase to  {0} " (`|GetEnumeratorNameAsString` InputState))))
  (bind _asbp_mjaiboss_aictg (cast `/Game/TG/AI/BP_MJAIBossAICTG` (`AIBlueprintHelperLibrary.GetAIController` _returnvalue))
    (:`then`
      (`BlackboardComponent.SetValueAsEnum` (`AIController.Blackboard` _asbp_mjaiboss_aictg) (`self.BossStateKey`) InputState))
    (:`CastFailed`
      (`KismetSystemLibrary.PrintText` "Cast Failed"))))

(fn `UserConstructionScript`)