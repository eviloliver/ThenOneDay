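; Test portal actor in the town that sends the player into the dungeon when something overlaps its collision.
; It reads the current dungeon map number from the game instance's session data and looks up that node in the dungeon generation subsystem's graph.
; The node type picks a Battle, Reward or Boss chunk map, with Battle names built from the assigned map ID, and the town game mode travels there with the node ID.
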(event `self.Collision.OnComponentBeginOverlap`
  (params (OverlappedComponent :type "PrimitiveComponent Object Reference") (OtherActor :type "Actor Object Reference") (OtherComp :type "PrimitiveComponent Object Reference") (OtherBodyIndex :type Integer) (bFromSweep :type Boolean) (SweepResult :type "HitResult Structure (by ref)"))
  (`|ExecutionSequence`
    (:`then_0`
      (bind _asbp_gamemode_town_tg (cast `/Game/Core/GameMode/BP_Gamemode_Town_TG` (`GameplayStatics.GetGameMode`)))
      (bind _asmjgame_instance_tg (cast `MJGameInstanceTG` (`GameplayStatics.GetGameInstance`))
        (:`then`
          (`KismetSystemLibrary.PrintText` "Travel to DugeonStartnode!!" true true (struct :`R` 1.0 :`G` 0.073746 :`A` 1.0))
          (bind _returnvalue (`MJGameInstanceTG.GetPlayerSessionDataRef` _asmjgame_instance_tg))
          (bind (_nodeid _assignedmapid _nodetype) (break `DungeonNode` (`|GetArrayItem` (`.Nodes` (break `DungeonGraph` (`MJDungeonGenerationSubSystem.DungeonGraph` (subsystem `MJDungeonGenerationSubSystem`)))) (`KismetMathLibrary.Conv_ByteToInt` (`.CurrentDungeonMapNum` (break `MJPlayerSessionData` _returnvalue))))))
          (switch `ENodeType` _nodetype
            (:`Battle`
              (`MJGameModeBase.TravelToMapByNode` _asbp_gamemode_town_tg (`KismetTextLibrary.Conv_TextToString` (`|FormatText` "Dungeon_Chunk_Battle0{0}" (`KismetMathLibrary.Conv_IntToByte` _assignedmapid))) (`KismetMathLibrary.Conv_IntToByte` _nodeid)))
            (:`Reward`
              (`MJGameModeBase.TravelToMapByNode` _asbp_gamemode_town_tg (`KismetTextLibrary.Conv_TextToString` (`|FormatText` "Dungeon_Chunk_Reward")) (`KismetMathLibrary.Conv_IntToByte` _nodeid)))
            (:`Boss`
              (`MJGameModeBase.TravelToMapByNode` _asbp_gamemode_town_tg (`KismetTextLibrary.Conv_TextToString` (`|FormatText` "Dungeon_Chunk_Boss")) (`KismetMathLibrary.Conv_IntToByte` _nodeid)))))
        (:`CastFailed`
          (`KismetSystemLibrary.PrintText` "Cast Failed!"))))))

(fn `UserConstructionScript`)