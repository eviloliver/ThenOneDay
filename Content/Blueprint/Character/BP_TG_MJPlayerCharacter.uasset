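; Test player character Blueprint with debug keys for a dungeon map and dummy actor spawning.
; M toggles a flag that either creates the dungeon map test widget on the MJ player controller and draws its graph, or removes it from the viewport.
; E spawns a TG dummy actor a short distance in front of the character along the control rotation.
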(event `Key|M`
  (params (Key :type "Key Structure"))
  (:`Pressed`
    (bind _output_get (set `self.MapButtonPressed` (not (`self.MapButtonPressed`))))
    (if _output_get
      (bind _asbp_mjplayer_controller (cast `/Game/Assets/Blueprint/Controller/BP_MJPlayerController` (`self.GetController` self)))
      (bind _returnvalue (`|CreateWidget` "/Game/Blueprint/WBP_DungeonMapTest.WBP_DungeonMapTest_C" _asbp_mjplayer_controller))
      (`UserWidget.AddToViewport` _returnvalue 0)
      (`/Game/Blueprint/WBP_DungeonMapTest.DrawGraph` _returnvalue)
      (else
        (`Widget.RemoveFromParent` _returnvalue)))))

(event `Key|E`
  (params (Key :type "Key Structure"))
  (:`Pressed`
    (`|SpawnActorFromClass` "/Game/Blueprint/BP_DummyActor_TG.BP_DummyActor_TG_C" (`KismetMathLibrary.Conv_VectorToTransform` (+ (`self.K2_GetActorLocation`) (* (`KismetMathLibrary.GetForwardVector` (`self.GetControlRotation`)) 100.0))) "Undefined" "MultiplyWithRoot" null null)))

(fn `UserConstructionScript`)