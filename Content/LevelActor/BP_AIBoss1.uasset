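; BP_AIBoss1 is a dungeon AI boss that tracks its health and performs melee attacks.
; One tick after BeginPlay, it publishes its spawn and current health through BP_GameState_Dungeon and binds to that state's boss health-change event.
; That event subtracts the received delta from current health, with no clamping or death handling here.
; MeleeAttack plays a supplied montage and signals attack end on completion or interruption.
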(event `self.ReceiveBeginPlay`
  (`KismetSystemLibrary.PrintText` "AiBoss Beginplay")
  (`KismetSystemLibrary.DelayUntilNextTick`)
  (bind _asbp_game_state_dungeon (cast `/Game/Core/GameState/BP_GameState_Dungeon` (`GameplayStatics.GetGameState`)))
  (`MJGameStateDungeonTG.PublishOnBossSpawned` _asbp_game_state_dungeon (`self.CurrHealth`))
  (add `MJGameStateDungeonTG.OnAIBossHealthChanged` _asbp_game_state_dungeon (delegate `OnHealthChanged`)))

(event `MeleeAttack`
  (params (InputAnimMontage :type "AnimMontage Object Reference"))
  (`|PlayMontage` (`self.Mesh`) InputAnimMontage
    (:`OnCompleted`
      _)
    (:`OnInterrupted`
      _))
  (`self.OnAttackEnd`))

(event `OnHealthChanged`
  (params (Delta :type "Float (single-precision)"))
  (set `self.CurrHealth` (- (`self.CurrHealth`) Delta)))

(fn `UserConstructionScript`)