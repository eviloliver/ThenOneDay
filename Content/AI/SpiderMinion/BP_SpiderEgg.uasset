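; Spider egg actor that hatches into a BP_SpiderCharacter on a short timer started at BeginPlay.
; When the timer fires, it sets the open flag on the body's MJAnimInstanceBase, plays a slime splash and spawns the spider just above the body, then destroys itself after a brief delay.
; If the anim instance cast fails, nothing hatches and the egg remains.
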(event `self.ReceiveBeginPlay`
  (`KismetSystemLibrary.K2_SetTimerDelegate` (delegate `커스텀이벤트`) 3.0))

(event `커스텀이벤트`
  (bind _body (`self.body`))
  (bind (_returnvalue_location _returnvalue_rotation) (`KismetMathLibrary.BreakTransform` (`SceneComponent.K2_GetComponentToWorld` _body)))
  (bind _asmjanim_instance_base (cast `MJAnimInstanceBase` (`SkeletalMeshComponent.GetAnimInstance` _body)))
  (`MJAnimInstanceBase.SetOpen` _asmjanim_instance_base true)
  (`GameplayStatics.SpawnEmitterAtLocation` "/Game/Enemy_Asset/SpiderMinion/Particles/P_SlimeSplash_01.P_SlimeSplash_01" _returnvalue_location _returnvalue_rotation (1.0 1.0 1.0) true "AutoRelease")
  (`|SpawnActorFromClass` "/Game/AI/SpiderMinion/BP_SpiderCharacter.BP_SpiderCharacter_C" (`KismetMathLibrary.MakeTransform` (+ _returnvalue_location (0.0 0.0 60.0)) _returnvalue_rotation) "AdjustIfPossibleButAlwaysSpawn" "MultiplyWithRoot" null null)
  (`KismetSystemLibrary.Delay` 1.0)
  (`self.K2_DestroyActor`))

(fn `UserConstructionScript`)