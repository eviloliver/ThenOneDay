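; Base monster character Blueprint that handles attack animation and movement speed.
; Attack plays an attack montage on the mesh and fires OnAttackEnd on completion or interruption.
; SetMovementSpeed maps a walking or sprinting state to the character's max walk speed and returns it.
; Appear is empty; its montage and OnAppearEnd chain is disconnected and never runs.
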(event `self.ReceiveBeginPlay`)

(event `Appear`)

(event `Attack`
  (`|PlayMontage` (`self.Mesh`) "/Game/Characters/Animation/Montage/AM_Attack_A.AM_Attack_A"
    (:`OnCompleted`
      _)
    (:`OnInterrupted`
      _))
  (`self.OnAttackEnd`))

(fn `SetMovementSpeed`
  (params (Speed :type "/Game/MJ/E_MovementSpeed Enum" :default "NewEnumerator0"))
  (returns (SpeedValue :type "Float (double-precision)"))
  (bind _output_get (set `CharacterMovementComponent.MaxWalkSpeed` (select `/Game/MJ/E_MovementSpeed` Speed :`NewEnumerator0` 200.0 :`NewEnumerator1` 400.0 :!type "Float (single-precision)") (`self.CharacterMovement`)))
  (return _output_get))

(fn `UserConstructionScript`)